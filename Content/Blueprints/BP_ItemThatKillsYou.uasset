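; A joke pickup item whose use actions quit the game, with on-screen text announcing each action.
; On pickup it attaches to the holder's skeletal mesh at an item socket and disables its box collision.
; On drop it detaches the cube and re-enables physics and collision at its current location.
; Primary use quits immediately, while secondary use quits after a five-second delay.
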(event `/Game/Blueprints/BPI_Item.Pickup`
  (params (SkeletalMesh :type "SkeletalMeshComponent Object Reference"))
  (`KismetSystemLibrary.PrintText` "Why did you pick this up")
  (`self.K2_AttachToComponent` SkeletalMesh "BPI_ItemSocket" "SnapToTarget" "SnapToTarget" "KeepRelative")
  (`PrimitiveComponent.SetCollisionEnabled` (`self.Box`) "NoCollision"))

(event `/Game/Blueprints/BPI_Item.Drop`
  (bind _cube (`self.Cube`))
  (`KismetSystemLibrary.PrintText` "Dropping")
  (set `self.Drop Location` (`SceneComponent.K2_GetComponentLocation` _cube))
  (`SceneComponent.K2_DetachFromComponent` _cube "KeepRelative" "KeepRelative" "KeepRelative" true)
  (`PrimitiveComponent.SetSimulatePhysics` (`self.Cube`) true)
  (`PrimitiveComponent.SetCollisionEnabled` (`self.Cube`) "QueryAndPhysics")
  (`SceneComponent.K2_SetWorldLocation` (`self.Cube`) (`self.Drop Location`) false false))

(event `/Game/Blueprints/BPI_Item.UsePrimary`
  (`KismetSystemLibrary.PrintText` "Die")
  (`KismetSystemLibrary.QuitGame` null "Quit"))

(event `/Game/Blueprints/BPI_Item.UseSecondary`
  (`KismetSystemLibrary.PrintText` "Die in 5 Seconds")
  (`KismetSystemLibrary.Delay` 5.0)
  (`KismetSystemLibrary.QuitGame` null "Quit"))

(fn `UserConstructionScript`)