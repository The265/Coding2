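; BP_EnemyBase is the base enemy character, providing melee attack, aggro, health and patrol functions.
; Attack plays a punch montage and immediately sphere-traces forward, damaging and reporting a damage event on the player, and calls AttackFinished on a hit or montage end.
; Aggro swaps the mesh to flat red, and lethal point damage triggers an impulse-driven ragdoll before destruction.
; Helpers set walk speed, return attack ranges and ping-pong along PatrolRoute spline points.
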(event `self.ReceiveBeginPlay`
  (set `self.Original_Material` (`PrimitiveComponent.GetMaterial` (`self.Mesh`) 0)))

(event `Attack`
  (bind _returnvalue (`self.K2_GetActorLocation`))
  (`KismetSystemLibrary.PrintText` "DIE")
  (`|PlayMontage` (`self.Mesh`) "/Game/CloseCombatAnimSet/Animations/InPlace/Attacks/NinjaLeftHook_Montage.NinjaLeftHook_Montage"
    (:`then`
      (bind (_bblockinghit _binitialoverlap _time _distance _location _impactpoint _normal _impactnormal _physmat _hitactor _hitcomponent _hitbonename _bonename _hititem _elementindex _faceindex _tracestart) (`GameplayStatics.BreakHitResult` (stale _outhit)))
      (`GameplayStatics.PlaySoundAtLocation` "/Game/SoundEffects/near-miss-swing-whoosh-5-233428.near-miss-swing-whoosh-5-233428" _tracestart (struct) 1.0 1.0 0.0 null null null null)
      (bind (_outhit _returnvalue_2) (`KismetSystemLibrary.SphereTraceSingle` :`Start` _returnvalue :`End` (+ _returnvalue (* (`self.GetActorForwardVector`) 100.0)) :`Radius` 50.0 :`TraceChannel` "TraceTypeQuery2" :`DrawDebugType` "ForDuration" :`DrawTime` 1.0))
      (if _returnvalue_2
        (bind _asbp_third_person_character (cast `/Game/ThirdPerson/Blueprints/BP_ThirdPersonCharacter` _hitactor))
        (`GameplayStatics.ApplyPointDamage` _asbp_third_person_character (`self.PunchDamage`) _tracestart _outhit (`self.GetController`))
        (`AISense_Damage.ReportDamageEvent` _asbp_third_person_character self 0.0 _tracestart)
        (`GameplayStatics.PlaySoundAtLocation` "/Game/SoundEffects/punch-04-383965.punch-04-383965" _tracestart (struct) 1.0 1.0 0.0 null null null null)
        (`self.AttackFinished` :!label _label)))
    (:`OnCompleted`
      (goto _label))
    (:`OnInterrupted`
      (goto _label))))

(event `GetAggroed`
  (`PrimitiveComponent.SetMaterial` (`self.Mesh`) 0 "/Game/Materials/MI_FlatRed.MI_FlatRed")
  (set `self.Aggroed` true))

(event `LoseAggro`
  (`PrimitiveComponent.SetMaterial` (`self.Mesh`) 0 (`self.Original_Material`))
  (set `self.Aggroed` false))

(event `SetWalkSpeed`
  (params (Speed :type "Float (double-precision)" :default 400.0))
  (set `CharacterMovementComponent.MaxWalkSpeed` Speed (`self.CharacterMovement`)))

(event `self.ReceivePointDamage`
  (params (Damage :type "Float (single-precision)") (DamageType :type "DamageType Object Reference") (HitLocation :type "Vector Structure") (HitNormal :type "Vector Structure") (HitComponent :type "PrimitiveComponent Object Reference") (BoneName :type Name) (ShotFromDirection :type "Vector Structure") (InstigatedBy :type "Controller Object Reference") (DamageCauser :type "Actor Object Reference") (HitInfo :type "HitResult Structure (by ref)"))
  (`KismetSystemLibrary.PrintText` (`|FormatText` "{instigator} hit me for {dmg} damage" InstigatedBy Damage))
  (set `self.Health` (- (`self.Health`) Damage))
  (if (<= (`self.Health`) 0.0)
    (`KismetSystemLibrary.PrintString` "Death")
    (`self.Ragdoll` ShotFromDirection)
    (`KismetSystemLibrary.Delay` 0.5)
    (`self.K2_DestroyActor`)))

(event `Ragdoll`
  (params (Origin :type "Vector Structure"))
  (`PrimitiveComponent.SetSimulatePhysics` (`self.Mesh`) true)
  (`PrimitiveComponent.AddRadialImpulse` (`self.Mesh`) (+ Origin (-100.0 0.0 0.0)) 300.0 100000.0 "RIF_Constant" false)
  (`CharacterMovementComponent.DisableMovement` (`self.CharacterMovement`)))

(fn `GetIdealRange`
  (returns (AttackRange :type "Float (double-precision)") (StrafeRange :type "Float (double-precision)"))
  (return (`self.Attack Range`) (`self.Strafe Range`)))

(fn `GetPatrolPointLocation`
  (returns (Location :type "Vector Structure"))
  (set `self.Patrol Index` (+ (`self.Patrol Index`) (`self.Direction`)))
  (if (>= (`self.Patrol Index`) (- (`SplineComponent.GetNumberOfSplinePoints` (`/Game/AI_Blueprints/BP_PatrolRoute.Spline` (`self.PatrolRoute`))) 1))
    (set `self.Direction` -1)
    (elif (<= (`self.Patrol Index`) 0)
      (set `self.Direction` 1)))
  (return (`SplineComponent.GetLocationAtSplinePoint` (`/Game/AI_Blueprints/BP_PatrolRoute.Spline` (`self.PatrolRoute`)) (`self.Patrol Index`) "World")))

(fn `UserConstructionScript`)