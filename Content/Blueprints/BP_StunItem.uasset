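; BP_StunItem is a carryable, single-use item that briefly stuns a nearby enemy.
; Pickup attaches it to a skeletal mesh socket and disables sphere collision, while Drop detaches it and restores physics and collision.
; UsePrimary sphere-traces PhysicsBody objects in place (zero-length offset) and deactivates the hit BP_EnemyBase's movement for a short delay.
; The item destroys itself after the stun or a miss, but remains if the hit actor fails the enemy cast.
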(event `/Game/Blueprints/BPI_Item.Pickup`
  (params (SkeletalMesh :type "SkeletalMeshComponent Object Reference"))
  (`KismetSystemLibrary.PrintText` "Stun Item is picked up")
  (`self.K2_AttachToComponent` SkeletalMesh "BPI_ItemSocket" "SnapToTarget" "SnapToTarget" "KeepRelative")
  (`PrimitiveComponent.SetCollisionEnabled` (`self.Sphere`) "NoCollision")
  (`GameplayStatics.PlaySound2D` "/Game/SoundEffects/plasticbag-77647.plasticbag-77647" 1.0 1.0 0.0 null null))

(event `/Game/Blueprints/BPI_Item.Drop`
  (bind _sphere (`self.Sphere`))
  (`KismetSystemLibrary.PrintText` "Dropping")
  (set `self.Drop Location` (`SceneComponent.K2_GetComponentLocation` _sphere))
  (`SceneComponent.K2_DetachFromComponent` _sphere "KeepRelative" "KeepRelative" "KeepRelative" true)
  (`PrimitiveComponent.SetSimulatePhysics` (`self.Sphere`) true)
  (`PrimitiveComponent.SetCollisionEnabled` (`self.Sphere`) "QueryAndPhysics")
  (`SceneComponent.K2_SetWorldLocation` (`self.Sphere`) (`self.Drop Location`) false false)
  (`GameplayStatics.PlaySound2D` "/Game/SoundEffects/luggage-drop-1-47660.luggage-drop-1-47660" 1.0 1.0 0.0 null null))

(event `/Game/Blueprints/BPI_Item.UsePrimary`
  (bind _sphere (`self.Sphere`))
  (bind _returnvalue (`SceneComponent.K2_GetComponentLocation` _sphere))
  (`GameplayStatics.PlaySound2D` "/Game/SoundEffects/lightening-bang-impact-40580.lightening-bang-impact-40580" 1.0 1.0 0.0 null null)
  (bind (_outhit _returnvalue_2) (`KismetSystemLibrary.SphereTraceSingleForObjects` :`Start` _returnvalue :`End` (+ _returnvalue (* (`KismetMathLibrary.GetForwardVector` (`SceneComponent.K2_GetComponentRotation` _sphere)) (0.0 0.0 0.0))) :`Radius` 250.0 :`ObjectTypes` (`|MakeArray` "ObjectTypeQuery4" :!type "EObjectTypeQuery Enum") :`DrawDebugType` "ForDuration"))
  (if _returnvalue_2
    (bind _asbp_enemy_base (cast `/Game/AI_Blueprints/BP_EnemyBase` (`.HitActor` (`GameplayStatics.BreakHitResult` _outhit))))
    (`KismetSystemLibrary.PrintString` "Hit Enemy")
    (bind _charactermovement (`Character.CharacterMovement` _asbp_enemy_base))
    (`ActorComponent.Deactivate` _charactermovement)
    (`KismetSystemLibrary.Delay` 1.5)
    (`ActorComponent.Activate` _charactermovement false)
    (`self.K2_DestroyActor`)
    (else
      (`self.K2_DestroyActor`))))

(fn `UserConstructionScript`)