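; Demo Blueprint for loops and lists that prints messages to the screen, starting on BeginPlay.
; DelayLoop re-calls itself after a one-second delay, capped by a DoN node whose count it prints, and runs StartForLoop on each pass.
; The for loop prints indices tinted from a color array.
; While and for-each variants are defined, but their calls are disconnected from execution.
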(event `self.ReceiveBeginPlay`
  (`KismetSystemLibrary.PrintString` "Loops and Lists is real")
  (`self.DelayLoop`))

(event `DelayLoop`
  (`KismetSystemLibrary.PrintText` (`|FormatText` "This has run {count} times" (stale _counter)))
  (`KismetSystemLibrary.Delay` 1.0)
  (bind _counter (`/Engine/EditorBlueprintResources/StandardMacros.Do N` 10)
    (:`Exit`
      (`self.StartForLoop`)
      (`self.DelayLoop`))))

(event `StartWhileLoop`
  (while (> (`self.WhileLoopCounter`) 0)
    (`KismetSystemLibrary.PrintText` (`|FormatText` "There are {uses} more uses in the loop" (`self.WhileLoopCounter`)) true true (struct :`G` 1.0 :`B` 0.030084 :`A` 1.0))
    (`/Engine/EditorBlueprintResources/StandardMacros.DecrementInt` (`self.WhileLoopCounter`)))
  (set `self.WhileLoopCounter` 10))

(event `StartForeachLoop`
  (for (_array_element _array_index) (`|MakeArray` (struct :`R` 1.0 :`G` 0.00905 :`A` 1.0) (struct :`R` 0.558036 :`G` 0.140902 :`B` 1.0 :`A` 1.0) (struct :`R` 1.0 :`G` 0.872805 :`A` 1.0) (struct :`R` 1.0 :`G` 0.001174 :`B` 0.170432 :`A` 1.0) :!type "LinearColor Structure")
    (`KismetSystemLibrary.PrintText` (`|FormatText` "This is Index # {index}" _array_index) true true _array_element)))

(event `StartForLoop`
  (bind _array (`|MakeArray` (struct :`R` 1.0 :`G` 0.00905 :`A` 1.0) (struct :`R` 0.558036 :`G` 0.140902 :`B` 1.0 :`A` 1.0) (struct :`R` 1.0 :`G` 0.872805 :`A` 1.0) (struct :`R` 1.0 :`G` 0.001174 :`B` 0.170432 :`A` 1.0) :!type "LinearColor Structure"))
  (for _index (range (`KismetArrayLibrary.Array_Length` _array))
    (`KismetSystemLibrary.PrintText` (`|FormatText` "This is Index # {index}" _index) true true (`|GetArrayItem` _array _index))))

(fn `UserConstructionScript`)