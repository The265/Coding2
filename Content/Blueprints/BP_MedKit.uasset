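; BP_MedKit is a held item, built from three cube meshes, that heals the player character.
; Pickup attaches it to a socket on the supplied skeletal mesh and disables collision; Drop detaches it and restores physics and collision.
; Primary use freezes player 0's movement for a short delay, applies HealAmount through ChangeHealth, destroys the kit, then restores walking.
; Each action plays a 2D sound.
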(event `/Game/Blueprints/BPI_Item.Pickup`
  (params (SkeletalMesh :type "SkeletalMeshComponent Object Reference"))
  (`KismetSystemLibrary.PrintText` "Stun Item is picked up")
  (`self.K2_AttachToComponent` SkeletalMesh "BPI_ItemSocket" "SnapToTarget" "SnapToTarget" "KeepRelative")
  (`PrimitiveComponent.SetCollisionEnabled` (`self.Cube`) "NoCollision")
  (`PrimitiveComponent.SetCollisionEnabled` (`self.Cube2`) "NoCollision")
  (`PrimitiveComponent.SetCollisionEnabled` (`self.Cube1`) "NoCollision")
  (`GameplayStatics.PlaySound2D` "/Game/SoundEffects/plasticbag-77647.plasticbag-77647" 1.0 1.0 0.0 null null))

(event `/Game/Blueprints/BPI_Item.Drop`
  (bind _cube (`self.Cube`))
  (`KismetSystemLibrary.PrintText` "Dropping")
  (set `self.Drop Location` (`SceneComponent.K2_GetComponentLocation` _cube))
  (`SceneComponent.K2_DetachFromComponent` _cube "KeepRelative" "KeepRelative" "KeepRelative" true)
  (`PrimitiveComponent.SetSimulatePhysics` (`self.Cube`) true)
  (`PrimitiveComponent.SetSimulatePhysics` (`self.Cube2`) true)
  (`PrimitiveComponent.SetSimulatePhysics` (`self.Cube1`) true)
  (`PrimitiveComponent.SetCollisionEnabled` (`self.Cube`) "QueryAndPhysics")
  (`PrimitiveComponent.SetCollisionEnabled` (`self.Cube2`) "QueryAndPhysics")
  (`PrimitiveComponent.SetCollisionEnabled` (`self.Cube1`) "QueryAndPhysics")
  (`SceneComponent.K2_SetWorldLocation` (`self.Cube`) (`self.Drop Location`) false false)
  (`SceneComponent.K2_SetWorldLocation` (`self.Cube2`) (`self.Drop Location`) false false)
  (`SceneComponent.K2_SetWorldLocation` (`self.Cube1`) (`self.Drop Location`) false false)
  (`GameplayStatics.PlaySound2D` "/Game/SoundEffects/luggage-drop-1-47660.luggage-drop-1-47660" 1.0 1.0 0.0 null null))

(event `/Game/Blueprints/BPI_Item.UsePrimary`
  (bind _asbp_third_person_character (cast `/Game/ThirdPerson/Blueprints/BP_ThirdPersonCharacter` (`GameplayStatics.GetPlayerCharacter` 0)))
  (`GameplayStatics.PlaySound2D` "/Game/SoundEffects/box-tape-210351.box-tape-210351" 1.0 1.0 0.0 null null)
  (`CharacterMovementComponent.DisableMovement` (`Character.CharacterMovement` _asbp_third_person_character))
  (`KismetSystemLibrary.Delay` 0.5)
  (`/Game/ThirdPerson/Blueprints/BP_ThirdPersonCharacter.ChangeHealth` _asbp_third_person_character (`self.Heal Amount`))
  (`self.K2_DestroyActor`)
  (`CharacterMovementComponent.SetMovementMode` (`Character.CharacterMovement` _asbp_third_person_character) "MOVE_Walking" 0))

(fn `UserConstructionScript`)