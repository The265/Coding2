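; Spawn manager that populates the level with AI enemies at every BP_EnemySpawnPoint when play begins.
; It gathers the spawn points, prints their count, then spawns a BP_AiMoveTo at each one, owned by that point; the weighted random check always passes.
; Each enemy gets a random text label, material and skeletal mesh, picked independently from arrays using hardcoded index ranges.
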(event `self.ReceiveBeginPlay`
  (bind _outactors (`GameplayStatics.GetAllActorsOfClass` "/Game/Blueprints/BP_EnemySpawnPoint.BP_EnemySpawnPoint_C"))
  (`KismetSystemLibrary.PrintText` (`|FormatText` "There are {count} spawn points in the level" (`KismetArrayLibrary.Array_Length` _outactors)))
  (for _array_element _outactors
    (if (`KismetMathLibrary.RandomBoolWithWeight` 100.0)
      (bind _returnvalue (`|SpawnActorFromClass` "/Game/AI_Blueprints/BP_AiMoveTo.BP_AiMoveTo_C" (`self.GetTransform` _array_element) "Undefined" "MultiplyWithRoot" _array_element null))
      (`TextRenderComponent.K2_SetText` (`/Game/AI_Blueprints/BP_AiMoveTo.TextRender` _returnvalue) (`KismetSystemLibrary.MakeLiteralText` (`|GetArrayItem` (`self.TextArray`) (`KismetMathLibrary.RandomIntegerInRange` 0 9))))
      (bind _mesh (`Character.Mesh` _returnvalue))
      (`PrimitiveComponent.SetMaterial` _mesh 0 (`|GetArrayItem` (`self.Material Array`) (`KismetMathLibrary.RandomIntegerInRange` 0 7)))
      (`SkeletalMeshComponent.SetSkeletalMeshAsset` _mesh (`|GetArrayItem` (`self.SkeletalArray`) (`KismetMathLibrary.RandomIntegerInRange` 0 7))))))

(fn `UserConstructionScript`)