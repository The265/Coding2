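; BP_Teletporter is a holdable teleporter item with pickup, drop, primary use and secondary use events.
; Pickup attaches it to a socket on the supplied skeletal mesh and disables box collision, while drop detaches the cube and enables physics.
; Primary use moves the third-person player character to a hard-coded location after a short delay.
; Secondary use announces a failed teleport, then destroys the item after a delay.
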(event `/Game/Blueprints/BPI_Item.Pickup`
  (params (SkeletalMesh :type "SkeletalMeshComponent Object Reference"))
  (`KismetSystemLibrary.PrintText` "This Teleporter is picked up")
  (`self.K2_AttachToComponent` SkeletalMesh "BPI_ItemSocket" "SnapToTarget" "SnapToTarget" "KeepRelative")
  (`PrimitiveComponent.SetCollisionEnabled` (`self.Box`) "NoCollision"))

(event `/Game/Blueprints/BPI_Item.Drop`
  (bind _cube (`self.Cube`))
  (`KismetSystemLibrary.PrintText` "Dropping")
  (set `self.Drop Location` (`SceneComponent.K2_GetComponentLocation` _cube))
  (`SceneComponent.K2_DetachFromComponent` _cube "KeepRelative" "KeepRelative" "KeepRelative" true)
  (`PrimitiveComponent.SetSimulatePhysics` (`self.Cube`) true)
  (`PrimitiveComponent.SetCollisionEnabled` (`self.Cube`) "QueryAndPhysics")
  (`SceneComponent.K2_SetWorldLocation` (`self.Cube`) (`self.Drop Location`) false false))

(event `/Game/Blueprints/BPI_Item.UsePrimary`
  (`KismetSystemLibrary.PrintText` "Teleporting")
  (`KismetSystemLibrary.Delay` 1.0)
  (bind _asbp_third_person_character (cast `/Game/ThirdPerson/Blueprints/BP_ThirdPersonCharacter` (`GameplayStatics.GetPlayerCharacter` 0)))
  (`self.K2_SetActorLocation` _asbp_third_person_character (2650.0 390.0 500.0) false false))

(event `/Game/Blueprints/BPI_Item.UseSecondary`
  (`KismetSystemLibrary.PrintText` "ERROR TELEPORT FAILED SELF DESTUCTION")
  (`KismetSystemLibrary.Delay` 5.0)
  (`self.K2_DestroyActor`))

(fn `UserConstructionScript`)